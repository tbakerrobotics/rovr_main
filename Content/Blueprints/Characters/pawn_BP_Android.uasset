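; Player pawn, named for Android, that moves along the camera's heading and interacts with widgets through a pointer.
; Forward input drives movement along the camera's yaw only, and the right grab action presses and releases a simulated left mouse button on the widget interaction component.
; On play start, the game instance's Android platform check sets that component's debug display flag.
; The construction script detaches the skeletal mesh.
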(event `InputAxis|MoveForward`
  (params (AxisValue :type "Float (single-precision)"))
  (bind (_returnvalue_roll _returnvalue_pitch _returnvalue_yaw) (`KismetMathLibrary.BreakRotator` (`SceneComponent.K2_GetComponentRotation` (`self.Camera`))))
  (`self.AddMovementInput` (`KismetMathLibrary.GetForwardVector` (`KismetMathLibrary.MakeRotator` 0.0 0.0 _returnvalue_yaw)) AxisValue))

(event `InputAction|GrabRight`
  (params (Key :type "Key Structure"))
  (bind _widgetinteraction (`self.WidgetInteraction`))
  (:`Pressed`
    (`WidgetInteractionComponent.PressPointerKey` _widgetinteraction "LeftMouseButton"))
  (:`Released`
    (`WidgetInteractionComponent.ReleasePointerKey` _widgetinteraction "LeftMouseButton")))

(event `self.ReceiveBeginPlay`
  (bind _asgame_info_instance (cast `/Game/Blueprints/AllLevels/gameInfoInstance` (`GameplayStatics.GetGameInstance`)))
  (set `WidgetInteractionComponent.bShowDebug` (`rovrGameInstance.androidPlatform_check` _asgame_info_instance) (`self.WidgetInteraction`)))

(fn `UserConstructionScript`
  (`SceneComponent.K2_DetachFromComponent` (`self.SkeletalMesh`) "KeepRelative" "KeepRelative" "KeepRelative" true))