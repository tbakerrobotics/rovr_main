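; Android player character base that handles forward movement and right-hand widget interaction.
; On BeginPlay it shows the right widget interaction debug display according to the game instance's Android platform check.
; MoveForward moves along the control yaw and prints the axis value each time it fires.
; GrabRight presses and releases a left-click on widgets, while DisplayNameTag is an empty stub.
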(event `self.ReceiveBeginPlay`
  (bind _asgame_info_instance (cast `/Game/Blueprints/AllLevels/gameInfoInstance` (`GameplayStatics.GetGameInstance`)))
  (set `WidgetInteractionComponent.bShowDebug` (`rovrGameInstance.androidPlatform_check` _asgame_info_instance) (`self.WidgetInteraction_R`)))

(event `InputAxis|MoveForward`
  (params (AxisValue :type "Float (single-precision)"))
  (bind (_returnvalue_roll _returnvalue_pitch _returnvalue_yaw) (`KismetMathLibrary.BreakRotator` (`self.GetControlRotation`)))
  (`KismetSystemLibrary.PrintString` (`KismetStringLibrary.Conv_DoubleToString` AxisValue))
  (`self.AddMovementInput` (`KismetMathLibrary.GetForwardVector` (`KismetMathLibrary.MakeRotator` 0.0 0.0 _returnvalue_yaw)) AxisValue))

(event `InputAction|GrabRight`
  (params (Key :type "Key Structure"))
  (bind _widgetinteraction_r (`self.WidgetInteraction_R`))
  (:`Pressed`
    (`WidgetInteractionComponent.PressPointerKey` _widgetinteraction_r "LeftMouseButton"))
  (:`Released`
    (`WidgetInteractionComponent.ReleasePointerKey` _widgetinteraction_r "LeftMouseButton")))

(fn `DisplayNameTag`)

(fn `UserConstructionScript`)