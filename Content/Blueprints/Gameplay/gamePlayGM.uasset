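; Gameplay game mode that spawns players as their selected characters and manages the multiplayer match roster.
; On controller swap it records the controller and copies server, audio and map info from the game instance.
; Respawning replaces the pawn at a random PlayerStart, matching the selection by display name to spawn an Android or PC variant.
; It also shares all player settings, triggers session destruction on logout and server-travels everyone back to the lobby.
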(event `self.ReceiveBeginPlay`)

(event `self.K2_OnSwapPlayerControllers`
  (params (OldPC :type "PlayerController Object Reference") (NewPC :type "PlayerController Object Reference"))
  ;[1 1 1] Keeps track of connecting player controllers
  (`KismetArrayLibrary.Array_Add` (`self.AllPlayerControllers`) NewPC)
  (bind _asgame_info_instance (cast `/Game/Blueprints/AllLevels/gameInfoInstance` (`GameplayStatics.GetGameInstance`))
    (:`then`
      (bind _asgameplay_pc (cast `/Game/Blueprints/Gameplay/gameplayPC` NewPC))
      (set `/Game/Blueprints/Gameplay/gameplayPC.ServerName` (`KismetTextLibrary.Conv_TextToString` (`/Game/Blueprints/AllLevels/gameInfoInstance.ServerName` _asgame_info_instance)) _asgameplay_pc)
      (set `/Game/Blueprints/Gameplay/gameplayPC.AudioType` (`/Game/Blueprints/AllLevels/gameInfoInstance.AudioType` _asgame_info_instance) _asgameplay_pc)
      (set `/Game/Blueprints/Gameplay/gameplayPC.MapImage` (`/Game/Blueprints/AllLevels/gameInfoInstance.MapImage` _asgame_info_instance) _asgameplay_pc)
      (set `/Game/Blueprints/Gameplay/gameplayPC.MapName` (`/Game/Blueprints/AllLevels/gameInfoInstance.MapName` _asgame_info_instance) _asgameplay_pc))
    (:`CastFailed`
      (`KismetSystemLibrary.PrintString` "CAST TO GAMEINFO FAILED" false true (struct :`G` 0.66 :`B` 1.0 :`A` 1.0) 5.0))))

(event `RespawnPlayer`
  (params (PlayerController :type "PlayerController Object Reference") (PlayerCharacter :type "Character Class Reference"))
  (bind _returnvalue (`Controller.K2_GetPawn` PlayerController))
  (bind _spawnpoints (`self.SpawnPoints`))
  ;[1 1 1] Spawn the player with the selected character from the gamplay PC
  (bind _outactors (`GameplayStatics.GetAllActorsOfClass` "/Script/Engine.PlayerStart"))
  (set `self.SpawnPoints` _outactors)
  (`/Engine/EditorBlueprintResources/StandardMacros.IsValid` _returnvalue
    (:`Is Valid`
      (`self.K2_DestroyActor` _returnvalue))
    (:`Is Not Valid`
      _))
  (`self.SpawnSelectedCharacter` PlayerController PlayerCharacter (`self.GetTransform` (`|GetArrayItem` _spawnpoints (`KismetMathLibrary.RandomIntegerInRange` 0 (- (`KismetArrayLibrary.Array_Length` _spawnpoints) 1))))))

(event `SpawnSelectedCharacter`
  (params (PlayerController :type "PlayerController Object Reference") (SelectedCharacter :type "Character Class Reference") (SpawnTransform :type "Transform Structure"))
  ;[1 1 1] Spawn and possess selected character. Spawn Actor does not allow only pawn inputs, so cannot verify that it is only pawn. Therefore, doesn't allow display name to be passed as a variable.
  (for (_array_element _array_index) (`self.AllCharacters`)
    (if (== (`KismetSystemLibrary.GetClassDisplayName` _array_element) (`KismetSystemLibrary.GetClassDisplayName` SelectedCharacter))
      (break)))
  (bind _asgameplay_pc (cast `/Game/Blueprints/Gameplay/gameplayPC` PlayerController)
    (:`then`
      (bind (_playersettings_myplayername _playersettings_myplayerimage _playersettings_myplayercharacter _playersettings_myplayercharacterimage _playersettings_myplayerstatus _playersettings_myplayerandroidcheck) (break `/Game/Blueprints/AllLevels/PlayerInfo` (`/Game/Blueprints/Gameplay/gameplayPC.PlayerSettings` _asgameplay_pc)))
      (if _playersettings_myplayerandroidcheck
        ;;[1 1 1] Spawns android version of character
        (switch `int` _array_index
          (:`0`
            (bind _returnvalue (`KismetTextLibrary.Conv_TextToString` _playersettings_myplayername))
            (bind _returnvalue_2 (`|SpawnActorFromClass` "/Game/Blueprints/Characters/base_0_Android.base_0_Android_C" SpawnTransform "Undefined" "OverrideRootScale" null _returnvalue null))
            (`Controller.Possess` PlayerController _returnvalue_2)
            (`KismetSystemLibrary.PrintString` "Spawned base character and possessed" false true (struct :`B` 1.0 :`A` 1.0) 5.0))
          (:`1`
            (bind _returnvalue_3 (`|SpawnActorFromClass` "/Game/Blueprints/Characters/carla_Android.carla_Android_C" SpawnTransform "Undefined" "OverrideRootScale" null _returnvalue null))
            (`KismetSystemLibrary.Delay` 0.1)
            (`Controller.Possess` PlayerController _returnvalue_3)
            (`KismetSystemLibrary.PrintString` "Spawned selected character and possessed" false true (struct :`R` 1.0 :`B` 0.768722 :`A` 1.0) 5.0 :!label _label))
          (:`2`
            (bind _returnvalue_4 (`|SpawnActorFromClass` "/Game/Blueprints/Characters/claudia_Android.claudia_Android_C" SpawnTransform "Undefined" "OverrideRootScale" null _returnvalue null))
            (`KismetSystemLibrary.Delay` 0.1)
            (`Controller.Possess` PlayerController _returnvalue_4)
            (goto _label))
          (:`3`
            (bind _returnvalue_5 (`|SpawnActorFromClass` "/Game/Blueprints/Characters/eric_Android.eric_Android_C" SpawnTransform "Undefined" "OverrideRootScale" null _returnvalue null))
            (`KismetSystemLibrary.Delay` 0.1)
            (`Controller.Possess` PlayerController _returnvalue_5)
            (goto _label))
          (:`4`
            (bind _returnvalue_6 (`|SpawnActorFromClass` "/Game/Blueprints/Characters/manuel_Android.manuel_Android_C" SpawnTransform "Undefined" "OverrideRootScale" null _returnvalue null))
            (`KismetSystemLibrary.Delay` 0.1)
            (`Controller.Possess` PlayerController _returnvalue_6)
            (goto _label))
          (:`5`
            (bind _returnvalue_7 (`|SpawnActorFromClass` "/Game/Blueprints/Characters/nathan_Android.nathan_Android_C" SpawnTransform "Undefined" "OverrideRootScale" null _returnvalue null))
            (`KismetSystemLibrary.Delay` 0.1)
            (`Controller.Possess` PlayerController _returnvalue_7)
            (goto _label))
          (:`6`
            (bind _returnvalue_8 (`|SpawnActorFromClass` "/Game/Blueprints/Characters/sophia_Android.sophia_Android_C" SpawnTransform "Undefined" "OverrideRootScale" null _returnvalue null))
            (`KismetSystemLibrary.Delay` 0.1)
            (`Controller.Possess` PlayerController _returnvalue_8)
            (goto _label)))
        (else
          ;;[1 1 1] Spawns PC version of character
          (switch `int` _array_index
            (:`0`
              (bind _returnvalue_9 (`KismetTextLibrary.Conv_TextToString` _playersettings_myplayername))
              (bind _returnvalue_10 (`|SpawnActorFromClass` "/Game/Blueprints/Characters/base_0.base_0_C" SpawnTransform "Undefined" "OverrideRootScale" null _returnvalue_9 null))
              (`Controller.Possess` PlayerController _returnvalue_10)
              (`KismetSystemLibrary.PrintString` (`KismetStringLibrary.Concat_StrStr` "Spawned base character and possessed. \nWith name: " _returnvalue_9) false true (struct :`B` 1.0 :`A` 1.0) 5.0))
            (:`1`
              (bind _returnvalue_11 (`|SpawnActorFromClass` "/Game/Blueprints/Characters/carla.carla_C" SpawnTransform "Undefined" "OverrideRootScale" null _returnvalue_9 null))
              (`KismetSystemLibrary.Delay` 0.1)
              (`Controller.Possess` PlayerController _returnvalue_11)
              (`KismetSystemLibrary.PrintString` "Spawned selected character and possessed" false true (struct :`R` 1.0 :`B` 0.768722 :`A` 1.0) 5.0 :!label _label_2))
            (:`2`
              (bind _returnvalue_12 (`|SpawnActorFromClass` "/Game/Blueprints/Characters/claudia.claudia_C" SpawnTransform "Undefined" "OverrideRootScale" null _returnvalue_9 null))
              (`KismetSystemLibrary.Delay` 0.1)
              (`Controller.Possess` PlayerController _returnvalue_12)
              (goto _label_2))
            (:`3`
              (bind _returnvalue_13 (`|SpawnActorFromClass` "/Game/Blueprints/Characters/eric.eric_C" SpawnTransform "Undefined" "OverrideRootScale" null _returnvalue_9 null))
              (`KismetSystemLibrary.Delay` 0.1)
              (`Controller.Possess` PlayerController _returnvalue_13)
              (goto _label_2))
            (:`4`
              (bind _returnvalue_14 (`|SpawnActorFromClass` "/Game/Blueprints/Characters/manuel.manuel_C" SpawnTransform "Undefined" "OverrideRootScale" null _returnvalue_9 null))
              (`KismetSystemLibrary.Delay` 0.1)
              (`Controller.Possess` PlayerController _returnvalue_14)
              (goto _label_2))
            (:`5`
              (bind _returnvalue_15 (`|SpawnActorFromClass` "/Game/Blueprints/Characters/nathan.nathan_C" SpawnTransform "Undefined" "OverrideRootScale" null _returnvalue_9 null))
              (`KismetSystemLibrary.Delay` 0.1)
              (`Controller.Possess` PlayerController _returnvalue_15)
              (goto _label_2))
            (:`6`
              (bind _returnvalue_16 (`|SpawnActorFromClass` "/Game/Blueprints/Characters/sophia.sophia_C" SpawnTransform "Undefined" "OverrideRootScale" null _returnvalue_9 null))
              (`KismetSystemLibrary.Delay` 0.1)
              (`Controller.Possess` PlayerController _returnvalue_16)
              (goto _label_2))))))
    (:`CastFailed`
      (`KismetSystemLibrary.PrintString` "CAST FAILED" false true (struct :`R` 1.0 :`G` 0.01752 :`A` 1.0) 10.0))))

(event `EveryoneAddPlayerInfo`
  (bind _allplayercontrollers (`self.AllPlayerControllers`))
  ;[1 1 1] Comment
  (`KismetArrayLibrary.Array_Clear` (`self.EveryonePlayerInfo`))
  (for _array_element _allplayercontrollers
    (bind _asgameplay_pc (cast `/Game/Blueprints/Gameplay/gameplayPC` _array_element))
    (`KismetArrayLibrary.Array_Add` (`self.EveryonePlayerInfo`) (`/Game/Blueprints/Gameplay/gameplayPC.PlayerSettings` _asgameplay_pc)))
  (for _array_element_2 _allplayercontrollers
    (bind _asgameplay_pc_2 (cast `/Game/Blueprints/Gameplay/gameplayPC` _array_element_2))
    (`/Game/Blueprints/Gameplay/gameplayPC.AddPlayerInfo` _asgameplay_pc_2 (`self.EveryonePlayerInfo`))))

(event `self.K2_OnLogout`
  (params (ExitingController :type "Controller Object Reference"))
  ;[1 1 1] Event on logout - destory session caller in game info instance
  (bind _asgameplay_pc (cast `/Game/Blueprints/Gameplay/gameplayPC` ExitingController))
  (`/Game/Blueprints/AllLevels/gameInfoInstance.DestroySessionCaller` (cast `/Game/Blueprints/AllLevels/gameInfoInstance` (`GameplayStatics.GetGameInstance`) :!pure true) _asgameplay_pc))

(event `ReturnToLobby`
  ;[1 1 1] Returns everyone to Lobby map
  (`KismetSystemLibrary.ExecuteConsoleCommand` "servertravel /Game/Maps/LobbyMap" (`GameplayStatics.GetPlayerController` 0)))

(fn `UserConstructionScript`)